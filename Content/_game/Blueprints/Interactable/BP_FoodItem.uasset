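; BP_FoodItem is an interactable food item that tracks a slicing state of Raw, Slicing or Sliced.
; SetState stores the new state and swaps the Sphere's material to match it, using stock-looking metal, floor and concrete materials.
; CanBeSliced reports true only when the item is flagged slicable and is not yet Sliced.
; BeginPlay, overlap and Tick are unused, disabled stubs.
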(event Custom|SetState
  (params (State :type BPE_FoodItemStates%20Enum :default "NewEnumerator0"))
  (bind _output_get (Variables|Default|SetState State))
  (Rendering|Material|SetMaterial (Variables|Default|GetSphere) 0 (Utilities|Select :Index _output_get :NewEnumerator0 "/Game/StarterContent/Materials/M_Metal_Copper.M_Metal_Copper" :NewEnumerator1 "/Game/StarterContent/Materials/M_Basic_Floor.M_Basic_Floor" :NewEnumerator2 "/Game/StarterContent/Materials/M_Concrete_Grime.M_Concrete_Grime")))

(event EventBeginPlay
  (|CallParentFunction) ; This node is disabled and will not be called.\nDrag off pins to build functionality.
)

(event Collision|EventActorBeginOverlap
  (params (OtherActor :type Actor%20Object%20Reference))
  (|CallParentFunction OtherActor) ; This node is disabled and will not be called.\nDrag off pins to build functionality.
)

(event EventTick
  (params (DeltaSeconds :type Float%20%28single-precision%29))
  (|CallParentFunction DeltaSeconds) ; This node is disabled and will not be called.\nDrag off pins to build functionality.
)

(fn ConstructionScript
  (|CallParentFunction))

(fn CanbeSliced
  (return (and (Variables|Default|GetIsSlicable) (Utilities|Select :Index (Variables|Default|GetState) :NewEnumerator0 true :NewEnumerator1 true :NewEnumerator2 false))))