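; BP_Table is an interactable table that holds one object the player places on it or picks up from it.
; GrabDrop hands a held object to AttachGrabbedObjectToTable, or gives the placed object to an empty-handed player.
; The attach function accepts an object only when the table is empty, then MoveComponentTo briefly animates it after attachment.
; The player's held reference clears even when the table is occupied.
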(event EventBeginPlay)

(event Collision|EventActorBeginOverlap
  (params (OtherActor :type Actor%20Object%20Reference)))

(event EventTick
  (params (DeltaSeconds :type Float%20%28single-precision%29)))

(event EventGrabDrop
  (params (Player :type BP%20Character%20Object%20Reference))
  (bind (_returnvalue _grabbedobject) (Default|GetGrabbedObject Player))
  ;[1 0.1302 0.1302 1 42] Handle Grab/Drop Event for BP_Table
  (if _returnvalue
    (bind _placedobject (CallFunction|AttachGrabbedObjecttoTable _grabbedobject))
    (Components|MoveComponentTo (Variables|/Script/Engine.Actor|GetRootComponent _placedobject) "0, 0, 0" "0, 0, 0" false false 0.05 false)
    (Variables|/Game/_game/Blueprints/BP_Character.BP_Character_C|SetGrabbedObject Player 0)
    (else
      (Utilities|IsValid (Variables|Default|GetPlacedObject)
        (:Is%20Valid
          (Default|Grab Player (Variables|Default|GetPlacedObject))
          (Variables|Default|SetPlacedObject 0))))))

(fn ConstructionScript)

(fn AttachGrabbedObjecttoTable
  (params (GrabbedObject :type BP%20Grabbable%20Object%20Reference))
  (Utilities|IsValid (Variables|Default|GetPlacedObject)
    (:Is%20Not%20Valid
      (bind _output_get (Variables|Default|SetPlacedObject GrabbedObject))
      (Transformation|AttachComponentToComponent _output_get (Variables|Default|GetTableTopAttachPoint) "None" "KeepWorld" "KeepWorld" "KeepWorld" true)
      (return (Variables|Default|GetPlacedObject)))))