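; Player character that moves along world axes, grabs and drops objects, and starts or stops interactions.
; Sphere traces just ahead, on separate channels for grab and interact, send messages to the hit actor.
; Grab attaches the object to Hands and moves it into place; pressing grab with no hit drops it.
; SetIsInteracting stores the interacting object and toggles an interaction input mapping context, while stop requests go to that object.
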(event Custom|SetIsInteracting
  (params (IsInteracting :type Boolean) (IsInteractingObject :type BPI%20Interactable%20Interface))
  (bind _returnvalue (Game|GetPlayerController 0))
  (bind _returnvalue_2 (PlayerController|LocalPlayerSubsystems|GetEnhancedInputLocalPlayerSubsystem _returnvalue))
  ;[0 1 0.1864] Input
  ;;[1 1 1 1 42] SetIsInteracting
  (Variables|Default|SetIsInteracting IsInteracting)
  (Variables|Default|SetInteractingObject IsInteractingObject)
  (if (Variables|Default|GetIsInteracting)
    (Input|AddMappingContext _returnvalue_2 "/Game/_game/Inputs/IMC_Interaction.IMC_Interaction" 0 "(bIgnoreAllPressedKeysUntilRelease=True,bForceImmediately=False,bNotifyUserSettings=False)")
    (else
      (Input|RemoveMappingContext _returnvalue_2 "/Game/_game/Inputs/IMC_Interaction.IMC_Interaction" "(bIgnoreAllPressedKeysUntilRelease=True,bForceImmediately=False,bNotifyUserSettings=False)"))))

(event Custom|Grab
  (params (ObjectToGrab :type BP%20Grabbable%20Object%20Reference))
  ;[1 1 1 1 32] Grab Invoked
  (bind _output_get (Variables|Default|SetGrabbedObject ObjectToGrab))
  (Transformation|AttachComponentToComponent _output_get (Variables|Default|GetHands) "None" "KeepWorld" "KeepWorld" "KeepWorld" true)
  (Components|MoveComponentTo (Variables|/Script/Engine.Actor|GetRootComponent (Variables|Default|GetGrabbedObject)) "0, 0, 0" "0, 0, 0" false false 0.2 false))

(event Custom|StopInteraction
  ;[1 1 1] StopInteraction
  (Default|StopInteraction (Variables|Default|GetInteractingObject)))

(event Input|EnhancedActionEvents|EnhancedInputActionIA_Movement
  (params (ActionValue :type Vector%202D%20Structure) (ElapsedSeconds :type Float%20%28double-precision%29) (TriggeredSeconds :type Float%20%28double-precision%29) (InputAction :type Input%20Action%20Object%20Reference :default "/Game/_game/Inputs/IA_Movement.IA_Movement"))
  ;[0 1 0.1864] Input
  ;;[1 1 1 1 42] Input: Movement
  (Pawn|Input|AddMovementInput (Math|Conversions|ToVector(Vector2D) ActionValue) 1.0 false))

(event Input|EnhancedActionEvents|EnhancedInputActionIA_StartInteraction
  (params (ActionValue :type Boolean) (ElapsedSeconds :type Float%20%28double-precision%29) (TriggeredSeconds :type Float%20%28double-precision%29) (InputAction :type Input%20Action%20Object%20Reference :default "/Game/_game/Inputs/IA_StartInteraction.IA_StartInteraction"))
  ;[0 1 0.1864] Input
  ;;[1 1 1 1 42] Input: StartInteraction
  (:Started
    (Development|PrintString "StartInteraction!")
    (if (Variables|Default|GetIsInteracting)
      (CallFunction|StopInteraction)
      (else
        (bind (_outhit _returnvalue) (CallFunction|FindObjecttoInteractwith "TraceTypeQuery4"))
        (if _returnvalue
          (Development|PrintString "Hit interactable objerct!")
          (Class|BPIInteractable|Interact(Message) (.HitActor (Collision|BreakHitResult _outhit)) self))))))

(event Input|EnhancedActionEvents|EnhancedInputActionIA_GrabDrop
  (params (ActionValue :type Boolean) (ElapsedSeconds :type Float%20%28double-precision%29) (TriggeredSeconds :type Float%20%28double-precision%29) (InputAction :type Input%20Action%20Object%20Reference :default "/Game/_game/Inputs/IA_GrabDrop.IA_GrabDrop"))
  (bind (_returnvalue _grabbedobject) (CallFunction|GetGrabbedObject))
  ;[0 1 0.1864] Input
  ;;[1 1 1 1 42] Input: GrabDrop
  (:Started
    (bind (_outhit _returnvalue_2) (CallFunction|FindObjecttoInteractwith "TraceTypeQuery3"))
    (if _returnvalue_2
      (Class|BPIInteractable|GrabDrop(Message) (.HitActor (Collision|BreakHitResult _outhit)) self)
      (elif _returnvalue
        (Default|Drop _grabbedobject)
        (Variables|Default|SetGrabbedObject 0)))))

(event Input|EnhancedActionEvents|EnhancedInputActionIA_StopInteraction
  (params (ActionValue :type Boolean) (ElapsedSeconds :type Float%20%28double-precision%29) (TriggeredSeconds :type Float%20%28double-precision%29) (InputAction :type Input%20Action%20Object%20Reference :default "/Game/_game/Inputs/IA_StopInteraction.IA_StopInteraction"))
  ;[1 1 1] StopInteraction
  (:Started
    (CallFunction|StopInteraction)))

(event EventBeginPlay)

(event Collision|EventActorBeginOverlap
  (params (OtherActor :type Actor%20Object%20Reference)))

(event EventTick
  (params (DeltaSeconds :type Float%20%28single-precision%29)))

(fn ConstructionScript)

(fn GetGrabbedObject
  (bind _grabbedobject (Variables|Default|GetGrabbedObject))
  (return (Utilities|IsValid _grabbedobject) _grabbedobject))

(fn DetermineAction
  (params (HitResult :type Hit%20Result%20Structure) (IsHit :type Boolean))
  (bind (_returnvalue _grabbedobject) (CallFunction|GetGrabbedObject))
  (if IsHit
    (Class|BPIInteractable|GrabDrop(Message) (.HitActor (Collision|BreakHitResult HitResult)) self)
    (elif _returnvalue
      (Default|Drop _grabbedobject)
      (Variables|Default|SetGrabbedObject 0))))

(fn FindObjecttoInteractwith
  (params (TraceChannel :type ETraceTypeQuery%20Enum :default "TraceTypeQuery1"))
  (bind _returnvalue (Transformation|GetActorLocation))
  (bind _returnvalue_2 (Transformation|GetActorForwardVector))
  (bind _returnvalue_3 (* _returnvalue_2 5e+01))
  (bind _returnvalue_4 (+ _returnvalue_3 _returnvalue))
  (bind (_x _y _z) (Math|Vector|BreakVector _returnvalue_4))
  (bind (_x_2 _y_2 _z_2) (Math|Vector|BreakVector _returnvalue_4))
  (bind (_outhit _returnvalue_5) (Collision|SphereTraceByChannel (Math|Vector|MakeVector _x _y (- _z 5e+01)) (Math|Vector|MakeVector _x_2 _y_2 (+ _z_2 1e+01)) 3e+01 TraceChannel false (Utilities|Array|MakeArray (Variables|Default|GetGrabbedObject)) "ForDuration"))
  (return _outhit _returnvalue_5))